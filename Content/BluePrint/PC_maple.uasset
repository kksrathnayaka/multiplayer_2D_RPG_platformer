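; Player controller that handles character selection and spawning of the chosen player character.
; On BeginPlay a client-prefixed event creates the character selection widget and adds it to the viewport.
; SelectCharacter forwards the chosen class and location through a server-prefixed event to the game mode as an interface-style spawn request message.
; A separate SpawnPlayer event spawns the given class at a transform and possesses it.
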(event `self.ReceiveBeginPlay`
  (`/Game/BluePrint/Interface/INT_PlayerController.InitializeWidgets`))

(event `/Game/BluePrint/Interface/INT_PlayerController.InitializeWidgets`
  (`self.CL_InitializeWidgets`))

(event `CL_InitializeWidgets`
  (bind _returnvalue (`|CreateWidget` "/Game/UI/WB_CharacterSection.WB_CharacterSection_C"))
  (bind _output_get (set `self.WB_CharacterSelection` _returnvalue))
  (`UserWidget.AddToViewport` _output_get 0))

(event `SRV_SelectCharacter`
  (params (Player :type "Actor Class Reference") (SpawnLocation :type "Vector Structure"))
  (bind _gamemode (message `/Game/BluePrint/Interface/INT_Gamemode.GetGameModeRef` (`GameplayStatics.GetGameMode`)))
  (message `/Game/BluePrint/Interface/INT_Gamemode.RequestSpawnPlayer` _gamemode self Player SpawnLocation))

(event `/Game/BluePrint/Interface/INT_PlayerController.SelectCharacter`
  (params (Player :type "Actor Class Reference") (SpawnLocation :type "Vector Structure"))
  (`self.SRV_SelectCharacter` Player SpawnLocation))

(event `/Game/BluePrint/Interface/INT_PlayerController.SpawnPlayer`
  (params (Player :type "Actor Class Reference") (SpawnTransform :type "Transform Structure"))
  (bind _returnvalue (`|SpawnActorFromClass` Player SpawnTransform "Undefined" "MultiplyWithRoot" null null))
  (bind _player (message `/Game/BluePrint/Interface/INT_Playerbase.GetPlayerRef` _returnvalue))
  (`self.Possess` _player))

(fn `GetPlayerControllerRef`
  (returns (PlayerController :type "/Game/BluePrint/PC_maple Object Reference"))
  (return self))

(fn `UserConstructionScript`)