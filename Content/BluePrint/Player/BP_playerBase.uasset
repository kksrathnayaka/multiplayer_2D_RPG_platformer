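; Base networked 2D player character with left/right running, jumping and flipbook animation.
; Movement input derives an Idle, Run, Jump or Fall state, sent via server event; its RepNotify swaps PlayerInfo flipbooks and rotates the sprite for facing.
; On BeginPlay, a server event fetches the spawn location from the GameMode, and its RepNotify moves the actor there.
; Jump sound is relayed through a server event to a multicast.
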(event `self.ReceiveBeginPlay`
  (`/Game/BluePrint/Interface/INT_Playerbase.SetPlayerSpawnLocation`))

(event `/Game/BluePrint/Interface/INT_Playerbase.SetPlayerSpawnLocation`
  (`self.SRV_SetPlayerSpawanLocation`))

(event `SRV_SetPlayerSpawanLocation`
  (bind _gamemode (message `/Game/BluePrint/Interface/INT_Gamemode.GetGameModeRef` (`GameplayStatics.GetGameMode`)))
  (set `self.Player Spawn Location` (`/Game/BluePrint/GM_Maple.PlayerSpawnLocation` _gamemode)))

(event `InputAxis|Move Right/Left`
  (params (AxisValue :type "Float (single-precision)"))
  ;[1 1 1] Player_Movement(Left and Right)
  (`self.AddMovementInput` (`KismetMathLibrary.GetForwardVector` (`self.GetControlRotation`)) AxisValue)
  (if (`NavMovementComponent.IsFalling` (`self.CharacterMovement`))
    (if (> (.z (`self.GetVelocity`)) 0.0)
      (`/Game/BluePrint/Interface/INT_Playerbase.SetMovementState` "NewEnumerator3")
      (else
        (`/Game/BluePrint/Interface/INT_Playerbase.SetMovementState` "NewEnumerator4")))
    (elif (== AxisValue 0.0)
      (`/Game/BluePrint/Interface/INT_Playerbase.SetMovementState` "NewEnumerator0")
      (elif (> AxisValue 0.0)
        (`/Game/BluePrint/Interface/INT_Playerbase.SetMovementState` "NewEnumerator1")
        (else
          (`/Game/BluePrint/Interface/INT_Playerbase.SetMovementState` "NewEnumerator2"))))))

(event `/Game/BluePrint/Interface/INT_Playerbase.SetMovementState`
  (params (MovementState :type "/Game/BluePrint/Enums/E_MovementState Enum" :default "NewEnumerator0"))
  ;[1 1 1] Player_Movement(Left and Right)
  (`self.SRV_SetMOvementState` MovementState))

(event `SRV_SetMOvementState`
  (params (MovementState :type "/Game/BluePrint/Enums/E_MovementState Enum" :default "NewEnumerator0"))
  ;[1 1 1] Player_Movement(Left and Right)
  (set `self.MovementState` MovementState))

(event `InputAction|Jump`
  (params (Key :type "Key Structure"))
  ;[1 1 1] Jump_Animation
  (:`Pressed`
    (if (`self.IsNotJumping`)
      (`self.Jump`)
      (`self.SRV_Jump` (`.JumpSfx_14_916EB0F946DAE267230864B601EF2A47` (break `/Game/BluePrint/Structs/ST_PlayeInfo` (`self.PlayerInfo`))) (`self.K2_GetActorLocation`)))))

(event `SRV_Jump`
  (params (`jump sfx` :type "SoundBase Object Reference") (playerlocation :type "Vector Structure"))
  ;[1 1 1] Jump_Animation
  (`self.MC_Jump` `jump sfx` playerlocation))

(event `MC_Jump`
  (params (`jump sfx` :type "SoundBase Object Reference") (playerlocation :type "Vector Structure"))
  ;[1 1 1] Jump_Animation
  (`GameplayStatics.PlaySoundAtLocation` `jump sfx` playerlocation (struct) 1.0 1.0 0.0 null null null null))

(fn `GetPlayerRef`
  (returns (Player :type "/Game/BluePrint/Player/BP_playerBase Object Reference"))
  (return self))

(fn `IsNotJumping`
  (returns (ReturnValue :type Boolean))
  (return (not (`NavMovementComponent.IsFalling` (`self.CharacterMovement`)))))

(fn `OnRep_MovementState`
  (bind (_idleanimation _runanimation _jumpaniamtion _fallanimation) (break `/Game/BluePrint/Structs/ST_PlayeInfo` (`self.PlayerInfo`)))
  (switch `/Game/BluePrint/Enums/E_MovementState` (`self.MovementState`)
    (:`NewEnumerator0`
      (`PaperFlipbookComponent.SetFlipbook` (`self.Sprite`) _idleanimation))
    (:`NewEnumerator1`
      (`SceneComponent.K2_SetRelativeRotation` :`self` (`self.Sprite`))
      (`PaperFlipbookComponent.SetFlipbook` (`self.Sprite`) _runanimation))
    (:`NewEnumerator2`
      (`SceneComponent.K2_SetRelativeRotation` (`self.Sprite`) (struct :`Yaw` 180.0) false false)
      (`PaperFlipbookComponent.SetFlipbook` (`self.Sprite`) _runanimation))
    (:`NewEnumerator3`
      (`PaperFlipbookComponent.SetFlipbook` (`self.Sprite`) _jumpaniamtion))
    (:`NewEnumerator4`
      (`PaperFlipbookComponent.SetFlipbook` (`self.Sprite`) _fallanimation))))

(fn `OnRep_Player Spawn Location`
  (`self.K2_SetActorLocation` (`self.Player Spawn Location`)))

(fn `UserConstructionScript`)